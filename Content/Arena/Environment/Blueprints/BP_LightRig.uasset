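; BP_LightRig is an arena light rig that sweeps a spotlight in a continuous moving pattern.
; Each Tick, two sine waves of game time at different rates drive pitch and yaw, with a Phase variable offsetting both.
; Spotlight brightness interpolates between a low and high level using the Intensity parameter from the MPC_Party material parameter collection.
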(event EventBeginPlay)

(event Collision|EventActorBeginOverlap
  (params (OtherActor :type Actor%20Object%20Reference)))

(event EventTick
  (params (DeltaSeconds :type Float%20%28single-precision%29))
  (Transformation|SetRelativeRotation (Variables|Default|GetSpotLight) (Math|Rotator|MakeRotator 0.0 (+ -6e+01 (* (Math|Trig|Sin(Radians) (+ (* (Utilities|Time|GetGameTimeinSeconds) 0.8) (Variables|Default|GetPhase))) 35.0)) (* (Math|Trig|Sin(Radians) (+ (* (Utilities|Time|GetGameTimeinSeconds) 0.6) (Variables|Default|GetPhase))) 5e+01)) false false)
  (bind _returnvalue (Rendering|Material|GetScalarParameterValue "/Game/Arena/Environment/Materials/MPC_Party.MPC_Party" "Intensity" :!class /Script/Engine.KismetMaterialLibrary))
  (Rendering|Components|Light|SetIntensity (Variables|Default|GetSpotLight) (Math|Float|Lerp 6e+04 1.5e+05 _returnvalue)))

(fn ConstructionScript)