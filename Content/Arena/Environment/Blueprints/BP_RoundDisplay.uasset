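; BP_RoundDisplay is an in-world arena display showing the game phase and round as main and sub text.
; It binds to the GameFlowManager's state change, setting both texts and a shared DisplayColor in the MPC_Party material parameter collection for tutorial, build, combat and game-over states.
; A separate ShowText event takes custom text and color, recolors the Glow light, and plays an Arrival timeline driving DisplayFlash and main-text scale.
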(event Custom|ShowText
  (params (Main :type Text) (Sub :type Text) (Color :type Linear%20Color%20Structure))
  (Rendering|Components|TextRender|SetText (Variables|Default|GetMainText) Main)
  (Rendering|Components|TextRender|SetText (Variables|Default|GetSubText) Sub)
  (Rendering|Material|SetVectorParameterValue "/Game/Arena/Environment/Materials/MPC_Party.MPC_Party" "DisplayColor" Color :!class /Script/Engine.KismetMaterialLibrary)
  (Rendering|Components|Light|SetLightColor (Variables|Default|GetGlow) Color true)
  (bind _alpha (Timeline|Arrival PlayFromStart)
    (:Update
      (Rendering|Material|SetScalarParameterValue "/Game/Arena/Environment/Materials/MPC_Party.MPC_Party" "DisplayFlash" _alpha :!class /Script/Engine.KismetMaterialLibrary)
      (Transformation|SetRelativeScale3D (Variables|Default|GetMainText) (Math|Vector|MakeVector (Math|Float|Lerp 1.0 1.3 _alpha) (Math|Float|Lerp 1.0 1.3 _alpha) (Math|Float|Lerp 1.0 1.3 _alpha))))))

(event Custom|OnStateChanged_Event
  (params (NewState :type EGameFlowState%20Enum :default "Idle") (PreviousState :type EGameFlowState%20Enum :default "Idle"))
  (switch Utilities|FlowControl|Switch|SwitchonEGameFlowState NewState
    (:TutorialCombat
      (Rendering|Components|TextRender|SetText (Variables|Default|GetMainText) (Utilities|Text|FormatText "TUTORIAL"))
      (Rendering|Components|TextRender|SetText (Variables|Default|GetSubText) (Utilities|Text|FormatText "COMBAT"))
      (Rendering|Material|SetVectorParameterValue "/Game/Arena/Environment/Materials/MPC_Party.MPC_Party" "DisplayColor" (Math|Color|MakeColor 0.0 1.0 1.0) :!class /Script/Engine.KismetMaterialLibrary))
    (:TutorialBuild
      (Rendering|Components|TextRender|SetText (Variables|Default|GetMainText) (Utilities|Text|FormatText "TUTORIAL"))
      (Rendering|Components|TextRender|SetText (Variables|Default|GetSubText) (Utilities|Text|FormatText "BUILD"))
      (Rendering|Material|SetVectorParameterValue "/Game/Arena/Environment/Materials/MPC_Party.MPC_Party" "DisplayColor" (Math|Color|MakeColor 0.0 1.0 1.0) :!class /Script/Engine.KismetMaterialLibrary))
    (:Build
      (Rendering|Components|TextRender|SetText (Variables|Default|GetMainText) (Utilities|Text|FormatText "ROUND {0}" (+ (Class|GameFlowManager|GetRoundsWon (Variables|Default|GetFlowManager)) 1)))
      (Rendering|Components|TextRender|SetText (Variables|Default|GetSubText) (Utilities|Text|FormatText "BUILD PHASE"))
      (Rendering|Material|SetVectorParameterValue "/Game/Arena/Environment/Materials/MPC_Party.MPC_Party" "DisplayColor" (Math|Color|MakeColor 0.5 1.0 0.2) :!class /Script/Engine.KismetMaterialLibrary))
    (:RoundCombat
      (Rendering|Components|TextRender|SetText (Variables|Default|GetMainText) (Utilities|Text|FormatText "ROUND {0}" (Class|GameFlowManager|GetCurrentRound (Variables|Default|GetFlowManager))))
      (Rendering|Components|TextRender|SetText (Variables|Default|GetSubText) (Utilities|Text|FormatText "FIGHT!"))
      (Rendering|Material|SetVectorParameterValue "/Game/Arena/Environment/Materials/MPC_Party.MPC_Party" "DisplayColor" (Math|Color|MakeColor 1.0 0.1 0.8) :!class /Script/Engine.KismetMaterialLibrary))
    (:GameOver
      (Rendering|Components|TextRender|SetText (Variables|Default|GetMainText) (Utilities|Text|FormatText "GAME OVER"))
      (Rendering|Components|TextRender|SetText (Variables|Default|GetSubText) (Utilities|Text|FormatText "{RoundsWon} ROUNDS WON!" (Class|GameFlowManager|GetRoundsWon (Variables|Default|GetFlowManager))))
      (Rendering|Material|SetVectorParameterValue "/Game/Arena/Environment/Materials/MPC_Party.MPC_Party" "DisplayColor" (Math|Color|MakeColor 1.0 0.1 0.1) :!class /Script/Engine.KismetMaterialLibrary))))

(event EventBeginPlay
  (bind _returnvalue (Actor|GetActorOfClass "/Script/Sparring_Protocol.GameFlowManager"))
  (Utilities|IsValid _returnvalue
    (:Is%20Valid
      (bind _output_get (Variables|Default|SetFlowManager _returnvalue))
      (EventDispatchers|AssignOnStateChanged _output_get (delegate Custom|OnStateChanged_Event)))))

(event Collision|EventActorBeginOverlap
  (params (OtherActor :type Actor%20Object%20Reference)))

(event EventTick
  (params (DeltaSeconds :type Float%20%28single-precision%29)))

(fn ConstructionScript)